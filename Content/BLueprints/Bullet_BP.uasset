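; Bullet actor that is launched by a physics force and reacts to hitting a Target_BP.
; Initialize pushes the Body component along the Sphere component's forward vector, scaled by the supplied force.
; The first overlap between Body and a Target_BP passes a DoOnce gate, spawns a rainbow flash particle at Body's location, then destroys the bullet after a short delay.
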(event OnComponentBeginOverlap(Body)
  (params (OtherActor :type Actor%20Object%20Reference) (OtherComp :type Primitive%20Component%20Object%20Reference) (OtherBodyIndex :type Integer) (bFromSweep :type Boolean) (SweepResult :type Hit%20Result%20Structure%20%28by%20ref%29))
  (Utilities|Casting|CastToTarget_BP OtherActor)
  (Utilities|FlowControl|DoOnce false
    (:Completed
      (Effects|SpawnEmitteratLocation "/Game/KY_MagicEffects01/Particles/P_rainbowFlash.P_rainbowFlash" (Transformation|GetWorldLocation (Variables|Default|GetBody)))
      (Utilities|FlowControl|Delay 2.0)
      (Actor|DestroyActor))))

(fn ConstructionScript)

(fn Initialize
  (params (Force :type Float%20%28single-precision%29))
  (bind _sphere (Variables|Default|GetSphere))
  (bind _returnvalue (Math|Vector|GetForwardVector _sphere))
  (Physics|AddForce (Variables|Default|GetBody) (Math|Vector|MakeVector (* Force (.x _returnvalue)) (* Force (.y _returnvalue)) (* Force (.z _returnvalue))) "None" false))