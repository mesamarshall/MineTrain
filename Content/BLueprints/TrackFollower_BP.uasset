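; TrackFollower_BP is an actor that rides along a referenced Track's spline, started by pressing Space Bar.
; Each Tick, constant interpolation ramps CurrentSpeed toward TargetSpeed when Active, or toward zero otherwise.
; Speed is added to the track distance per frame, without delta-time scaling, then sets location and rotation from the spline.
; Distance resets to zero at the spline's end, looping the ride.
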(event EventBeginPlay)

(event EventActorBeginOverlap
  (params (OtherActor :type Actor%20Object%20Reference)))

(event EventTick
  (params (DeltaSeconds :type Float%20%28single-precision%29))
  (if (Variables|Default|GetActive)
    (Variables|Default|SetCurrentSpeed (Math|Interpolation|FInterptoConstant (Variables|Default|GetCurrentSpeed) (Variables|Default|GetTargetSpeed) (Utilities|Time|GetWorldDeltaSeconds) (Variables|Default|GetAcceleration)))
    (else
      (Variables|Default|SetCurrentSpeed (Math|Interpolation|FInterptoConstant (Variables|Default|GetCurrentSpeed) 0.0 (Utilities|Time|GetWorldDeltaSeconds) (Variables|Default|GetAcceleration)))))
  (Variables|Default|SetPositionOnTrack (+ (Variables|Default|GetPositionOnTrack) (Variables|Default|GetCurrentSpeed)))
  (Transformation|SetActorLocation (Spline|GetLocationatDistanceAlongSpline (Variables|/Game/BLueprints/Track_BP.Track_BP_C|GetSpline (Variables|Default|GetTrack)) (Variables|Default|GetPositionOnTrack) "World") false false)
  (Transformation|SetActorRotation (Spline|GetRotationatDistanceAlongSpline (Variables|/Game/BLueprints/Track_BP.Track_BP_C|GetSpline (Variables|Default|GetTrack)) (Variables|Default|GetPositionOnTrack) "World"))
  (if (>= (Variables|Default|GetPositionOnTrack) (Spline|GetSplineLength (Variables|/Game/BLueprints/Track_BP.Track_BP_C|GetSpline (Variables|Default|GetTrack))))
    (Variables|Default|SetPositionOnTrack 0.0)))

(event Input|KeyboardEvents|SpaceBar
  (params (Key :type Key%20Structure :default "AnyKey"))
  (:Pressed
    (CallFunction|StartonSpline)))

(fn ConstructionScript)

(fn StartonSpline
  (Variables|Default|SetActive true))